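; Base weapon Blueprint that supplies shared firing, ammo and sound logic, with empty shoot and stop events.
; Caches the first-person character, whose per-type ammo counts it checks and decrements, refreshing the matching HUD display.
; Offers hitscan firing via an object line trace that applies damage and spawns blood on "enemy"-tagged actors, or projectile firing that passes speed and damage to the spawned actor.
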(event `self.ReceiveBeginPlay`
  (bind _asbp_first_person_character (cast `/Game/FirstPerson/Blueprints/BP_FirstPersonCharacter` (`GameplayStatics.GetPlayerCharacter` 0)))
  (set `self.playercharacterref` _asbp_first_person_character))

(event `ShootWeapon`)

(event `StopShooting`)

(event `Decreaseammo`
  (bind _playercharacterref (`self.playercharacterref`))
  (bind _playercharacterref_2 (`self.playercharacterref`))
  (bind _playercharacterref_3 (`self.playercharacterref`))
  (bind _playercharacterref_4 (`self.playercharacterref`))
  (switch `/Game/Blueprints/Weapons/Ammo` (`self.ammotype`)
    (:`NewEnumerator0`
      (`/Engine/EditorBlueprintResources/StandardMacros.DecrementInt` (`/Game/FirstPerson/Blueprints/BP_FirstPersonCharacter.bullet` _playercharacterref_2)
        (:`  `
          (`/Game/Blueprints/UI/PlayerHUD.Updatebulletammo` (`/Game/FirstPerson/Blueprints/BP_FirstPersonCharacter.playerhud` _playercharacterref_2)))))
    (:`NewEnumerator1`
      (`/Engine/EditorBlueprintResources/StandardMacros.DecrementInt` (`/Game/FirstPerson/Blueprints/BP_FirstPersonCharacter.shell` _playercharacterref_3)
        (:`  `
          (`/Game/Blueprints/UI/PlayerHUD.UpdateShellamoo` (`/Game/FirstPerson/Blueprints/BP_FirstPersonCharacter.playerhud` _playercharacterref_3)))))
    (:`NewEnumerator2`
      (`/Engine/EditorBlueprintResources/StandardMacros.DecrementInt` (`/Game/FirstPerson/Blueprints/BP_FirstPersonCharacter.rock` _playercharacterref_4)
        (:`  `
          (`/Game/Blueprints/UI/PlayerHUD.Updaterocketammo` (`/Game/FirstPerson/Blueprints/BP_FirstPersonCharacter.playerhud` _playercharacterref_4)))))
    (:`NewEnumerator3`
      (`/Engine/EditorBlueprintResources/StandardMacros.DecrementInt` (`/Game/FirstPerson/Blueprints/BP_FirstPersonCharacter.cell` _playercharacterref)
        (:`  `
          (`/Game/Blueprints/UI/PlayerHUD.Updatecellammo` (`/Game/FirstPerson/Blueprints/BP_FirstPersonCharacter.playerhud` _playercharacterref)))))))

(event `Playweaponsound`
  (`GameplayStatics.PlaySoundAtLocation` (`self.Sound`) (`self.K2_GetActorLocation`) (struct) 1.0 1.0 0.0 null null null null))

(fn `Fireprojectile`
  (`|SpawnActorFromClass` (`self.projectile`) (`SceneComponent.K2_GetComponentToWorld` (`self.projectiletransform`)) "Undefined" "MultiplyWithRoot" null (`self.projectilespeed`) (`self.weapondamage`) null))

(fn `Fireweapon`
  (bind _returnvalue (`SceneComponent.K2_GetComponentLocation` (`self.linetrace`)))
  (bind (_outhit _returnvalue_2) (`KismetSystemLibrary.LineTraceSingleForObjects` _returnvalue (+ _returnvalue (* (`KismetMathLibrary.GetForwardVector` (`SceneComponent.K2_GetComponentRotation` (`self.linetrace`))) (`self.linetracedistance`))) (`|MakeArray` "ObjectTypeQuery1" "ObjectTypeQuery2" "ObjectTypeQuery3" :!type "EObjectTypeQuery Enum") false (`|MakeArray` self (`GameplayStatics.GetPlayerCharacter` 0) :!type "Actor Object Reference") "ForDuration"))
  (if _returnvalue_2
    (bind (_bblockinghit _binitialoverlap _time _distance _location _impactpoint _normal _impactnormal _physmat _hitactor) (`GameplayStatics.BreakHitResult` _outhit))
    (`GameplayStatics.ApplyDamage` _hitactor (`self.weapondamage`))
    (if (`self.ActorHasTag` _hitactor "enemy")
      (`|SpawnActorFromClass` "/Game/Enemies/Blood/Blood_BP.Blood_BP_C" (`KismetMathLibrary.MakeTransform` _location) "Undefined" "MultiplyWithRoot" null null))))

(fn `Hasenoughamoo?`
  (returns (hasammo :type Boolean))
  (switch `/Game/Blueprints/Weapons/Ammo` (`self.ammotype`)
    (:`NewEnumerator0`
      (if (> (`/Game/FirstPerson/Blueprints/BP_FirstPersonCharacter.bullet` (`self.playercharacterref`)) 0)
        (return true)
        (else
          (return false))))
    (:`NewEnumerator1`
      (if (> (`/Game/FirstPerson/Blueprints/BP_FirstPersonCharacter.shell` (`self.playercharacterref`)) 0)
        (return true)
        (else
          (return false))))
    (:`NewEnumerator2`
      (if (> (`/Game/FirstPerson/Blueprints/BP_FirstPersonCharacter.rock` (`self.playercharacterref`)) 0)
        (return true)
        (else
          (return false))))
    (:`NewEnumerator3`
      (if (> (`/Game/FirstPerson/Blueprints/BP_FirstPersonCharacter.cell` (`self.playercharacterref`)) 0)
        (return true)
        (else
          (return false))))))

(fn `UserConstructionScript`)