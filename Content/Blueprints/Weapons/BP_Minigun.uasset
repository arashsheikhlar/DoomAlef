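; Minigun weapon Blueprint that fires continuously while shooting is active.
; ShootWeapon uses a DoOnce gate to start a looping timer that calls the fire event at a fixed interval.
; Each tick checks ammo, then consumes it, fires, plays sound and shows the firing flipbook.
; Running out of ammo or StopShooting clears the timer, switches to the idle flipbook and resets the gate.
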(event `self.ShootWeapon`
  (`/Engine/EditorBlueprintResources/StandardMacros.DoOnce` false :!label _label
    (:`Completed`
      (bind _returnvalue (`KismetSystemLibrary.K2_SetTimerDelegate` (delegate `fireminigun`) 0.15 true))
      (set `self.minigunevent` _returnvalue))))

(event `resetfire`
  (goto _label :!via `Reset`))

(event `fireminigun`
  (`self.Hasenoughamoo?`)
  (if true
    (`self.Decreaseammo`)
    (`self.Fireweapon`)
    (`self.Playweaponsound`)
    (`PaperFlipbookComponent.SetFlipbook` (`self.Weaponflipbook`) "/Game/Sprites/Weapons/MiniGun/minigunfire.minigunfire")
    (else
      (`KismetSystemLibrary.K2_ClearAndInvalidateTimerHandle` (`self.minigunevent`) :!label _label_2)
      (`PaperFlipbookComponent.SetFlipbook` (`self.Weaponflipbook`) "/Game/Sprites/Weapons/MiniGun/minigunidle.minigunidle")
      (`self.resetfire`))))

(event `self.StopShooting`
  (goto _label_2))

(fn `UserConstructionScript`
  (`parent.UserConstructionScript`))