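; BP_Shotgun is a shotgun weapon that uses Paper2D flipbook animation for its idle and firing visuals.
; ShootWeapon checks for enough ammo, then passes a DoOnce gate to decrease ammo, fire, play the sound and switch to the fire flipbook.
; After a delay equal to that flipbook's length, it restores the idle flipbook and calls Resetfire to reopen the gate, so the animation length limits the fire rate.
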(event `self.ShootWeapon`
  (bind _weaponflipbook (`self.Weaponflipbook`))
  (bind _hasammo (`self.Hasenoughamoo?`))
  (if _hasammo
    (`/Engine/EditorBlueprintResources/StandardMacros.DoOnce` false :!label _label
      (:`Completed`
        (`self.Decreaseammo`)
        (`self.Fireweapon`)
        (`self.Playweaponsound`)
        (`PaperFlipbookComponent.SetFlipbook` _weaponflipbook "/Game/Sprites/Weapons/Shotgun/shotgunfire.shotgunfire")
        (`KismetSystemLibrary.Delay` (`PaperFlipbookComponent.GetFlipbookLength` _weaponflipbook))
        (`PaperFlipbookComponent.SetFlipbook` (`self.Weaponflipbook`) "/Game/Sprites/Weapons/Shotgun/shotgunidle.shotgunidle")
        (`self.Resetfire`)))))

(event `Resetfire`
  (goto _label :!via `Reset`))

(fn `UserConstructionScript`
  (`parent.UserConstructionScript`))