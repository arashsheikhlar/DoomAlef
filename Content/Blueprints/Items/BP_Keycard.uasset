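; BP_Keycard is a keycard pickup that comes in red, orange or blue, chosen by its Keycard variable.
; The construction script sets the matching Paper2D sprite, and Tick yaws the actor toward the player like a billboard.
; When BP_FirstPersonCharacter overlaps the box, it sets that character's matching keycard flag, notifies the player HUD and destroys the pickup.
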(event `self.Box.OnComponentBeginOverlap`
  (params (OverlappedComponent :type "PrimitiveComponent Object Reference") (OtherActor :type "Actor Object Reference") (OtherComp :type "PrimitiveComponent Object Reference") (OtherBodyIndex :type Integer) (bFromSweep :type Boolean) (SweepResult :type "HitResult Structure (by ref)"))
  (bind _firstpersoncharacterref (`self.firstpersoncharacterref`))
  (bind _firstpersoncharacterref_2 (`self.firstpersoncharacterref`))
  (bind _firstpersoncharacterref_3 (`self.firstpersoncharacterref`))
  (bind _asbp_first_person_character (cast `/Game/FirstPerson/Blueprints/BP_FirstPersonCharacter` OtherActor))
  (set `self.firstpersoncharacterref` _asbp_first_person_character)
  (switch `/Game/Blueprints/Items/Keycard` (`self.keycard`)
    (:`NewEnumerator0`
      (set `/Game/FirstPerson/Blueprints/BP_FirstPersonCharacter.redkeycard?` true _firstpersoncharacterref_2)
      (`/Game/Blueprints/UI/PlayerHUD.Findredkeycard` (`/Game/FirstPerson/Blueprints/BP_FirstPersonCharacter.playerhud` _firstpersoncharacterref_2)))
    (:`NewEnumerator1`
      (set `/Game/FirstPerson/Blueprints/BP_FirstPersonCharacter.orangekeycard?` true _firstpersoncharacterref_3)
      (`/Game/Blueprints/UI/PlayerHUD.Findorangekeycard` (`/Game/FirstPerson/Blueprints/BP_FirstPersonCharacter.playerhud` _firstpersoncharacterref_3)))
    (:`NewEnumerator2`
      (set `/Game/FirstPerson/Blueprints/BP_FirstPersonCharacter.bluekeycard?` true _firstpersoncharacterref)
      (`/Game/Blueprints/UI/PlayerHUD.Findbluekeycard` (`/Game/FirstPerson/Blueprints/BP_FirstPersonCharacter.playerhud` _firstpersoncharacterref))))
  (`self.K2_DestroyActor`))

(event `self.ReceiveTick`
  (params (DeltaSeconds :type "Float (single-precision)"))
  (bind (_returnvalue_roll _returnvalue_pitch _returnvalue_yaw) (`KismetMathLibrary.BreakRotator` (`KismetMathLibrary.FindLookAtRotation` (`self.K2_GetActorLocation`) (`self.K2_GetActorLocation` (`GameplayStatics.GetPlayerCharacter` 0)))))
  (`self.K2_SetActorRotation` (`KismetMathLibrary.MakeRotator` 0.0 0.0 _returnvalue_yaw)))

(fn `UserConstructionScript`
  (switch `/Game/Blueprints/Items/Keycard` (`self.keycard`)
    (:`NewEnumerator0`
      (`PaperSpriteComponent.SetSprite` (`self.PaperSprite`) "/Game/Sprites/Items/redkey_sprite.redkey_sprite"))
    (:`NewEnumerator1`
      (`PaperSpriteComponent.SetSprite` (`self.PaperSprite`) "/Game/Sprites/Items/orangekey_sprite.orangekey_sprite"))
    (:`NewEnumerator2`
      (`PaperSpriteComponent.SetSprite` (`self.PaperSprite`) "/Game/Sprites/Items/bluekey_sprite.bluekey_sprite"))))